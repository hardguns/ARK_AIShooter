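; Enemy character Blueprint that shows its current health as colored in-world text.
; On BeginPlay and whenever HealthComponent reports a health change, it updates HealthText with the value and a healthy, hurt or critical color chosen by fixed thresholds.
; When HealthComponent signals death, it hides the text.
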(event `self.ReceiveBeginPlay`
  (`self.SetHealthTextProperties` (`STS_HealthComponent.CurrentHealth` (`self.HealthComponent`))))

(event `self.HealthComponent.OnHealthChanged`
  (params (HealthComponent :type "STS_HealthComponent Object Reference") (Health :type "Float (single-precision)") (HealthDelta :type "Float (single-precision)") (DamageType :type "DamageType Object Reference") (InstigatedBy :type "Controller Object Reference") (DamageCauser :type "Actor Object Reference"))
  (`self.SetHealthTextProperties` Health))

(event `self.HealthComponent.OnDeath`
  (params (HealthComponent :type "STS_HealthComponent Object Reference") (InstigatedBy :type "Controller Object Reference") (Killer :type "Actor Object Reference"))
  (`SceneComponent.SetVisibility` (`self.HealthText`) false false))

(fn `GetColorFromHealth`
  (params (Health :type "Float (double-precision)"))
  (returns (TextColor :type "Color Structure"))
  (if (>= Health 80.0)
    (return (`self.HealthyColor`))
    (elif (> Health 30.0)
      (return (`self.HurtColor`))
      (else
        (return (`self.CriticalColor`))))))

(fn `SetHealthTextProperties`
  (params (CurrentHealth :type "Float (double-precision)"))
  (bind _healthtext (`self.HealthText`))
  (`TextRenderComponent.K2_SetText` _healthtext (`KismetTextLibrary.Conv_DoubleToText` CurrentHealth "HalfToEven"))
  (`TextRenderComponent.SetTextRenderColor` _healthtext (`self.GetColorFromHealth` CurrentHealth)))

(fn `UserConstructionScript`)